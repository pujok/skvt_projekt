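; BP_SkvtScreen is an in-world screen actor that displays a WBP_SkvtWeb widget through its Webpage widget component.
; On BeginPlay, Initialize casts the component's widget and caches it as WebpageRef.
; TurnOff destroys the actor, while TurnOffEMP hides the webpage component and attaches a P_Sparks emitter to it, leaving the actor in place.
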(event `self.ReceiveBeginPlay`
  (`self.Initialize`))

(event `/Game/Skvt/Blueprints/BPI_ElectricDevice.TurnOff`
  (`self.K2_DestroyActor`))

(event `/Game/Skvt/Blueprints/BPI_ElectricDevice.TurnOffEMP`
  (bind _webpage (`self.Webpage`))
  (`SceneComponent.SetVisibility` _webpage false false)
  (`GameplayStatics.SpawnEmitterAttached` "/Game/StarterContent/Particles/P_Sparks.P_Sparks" _webpage "None" (`SceneComponent.GetSocketLocation` _webpage "None") (struct) (1.0 1.0 1.0) "KeepWorldPosition" false))

(fn `Initialize`
  (bind _aswbp_skvt_web (cast `/Game/Skvt/Blueprints/Screen/WBP_SkvtWeb` (`WidgetComponent.GetWidget` (`self.Webpage`))))
  (set `self.WebpageRef` _aswbp_skvt_web))

(fn `UserConstructionScript`)